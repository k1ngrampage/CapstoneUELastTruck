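; Placeholder pallet actor where the LastTruckPlayerPawn drops off packages by holding the Drop input.
; Box overlap enables input, shows a PalletWidget and opens a gate; leaving closes it and restores the PackageWidget.
; A held drop moves one package from LastTruckGameMode to Pallet1 after a retriggerable delay, spawning PHCompletePallet once full.
; A parallel timer, polled by a self-calling delay loop, feeds hold progress to the widget.
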(event `self.ReceiveHit`
  (params (MyComp :type "PrimitiveComponent Object Reference") (Other :type "Actor Object Reference") (OtherComp :type "PrimitiveComponent Object Reference") (bSelfMoved :type Boolean) (HitLocation :type "Vector Structure") (HitNormal :type "Vector Structure") (NormalImpulse :type "Vector Structure") (Hit :type "HitResult Structure (by ref)")))

(event `self.ReceiveActorBeginOverlap`
  (params (OtherActor :type "Actor Object Reference")))

(event `self.Box.OnComponentBeginOverlap`
  (params (OverlappedComponent :type "PrimitiveComponent Object Reference") (OtherActor :type "Actor Object Reference") (OtherComp :type "PrimitiveComponent Object Reference") (OtherBodyIndex :type Integer) (bFromSweep :type Boolean) (SweepResult :type "HitResult Structure (by ref)"))
  (cast `/Game/Blueprints/LastTruckPlayerPawn` OtherActor)
  (`self.EnableInput` (`GameplayStatics.GetPlayerController` 0))
  (bind _returnvalue (`|CreateWidget` "/Game/Widgets/PalletWidget.PalletWidget_C"))
  (bind _output_get (set `self.Widget` _returnvalue))
  (`UserWidget.AddToViewport` _output_get 0)
  (set `/Game/Widgets/PalletWidget.MaxTimeHeld` (`self.MaxHoldTime`) _output_get)
  (goto _label :!via `Open`))

(event `self.Box.OnComponentEndOverlap`
  (params (OverlappedComponent :type "PrimitiveComponent Object Reference") (OtherActor :type "Actor Object Reference") (OtherComp :type "PrimitiveComponent Object Reference") (OtherBodyIndex :type Integer))
  (cast `/Game/Blueprints/LastTruckPlayerPawn` OtherActor)
  (`self.DisableInput` (`GameplayStatics.GetPlayerController` 0))
  (`WidgetLayoutLibrary.RemoveAllWidgets`)
  (bind _returnvalue (`|CreateWidget` "/Game/Widgets/PackageWidget.PackageWidget_C"))
  (`UserWidget.AddToViewport` _returnvalue 0)
  (goto _label :!via `Close`))

(event `InputAction|Drop`
  (params (Key :type "Key Structure"))
  (:`Pressed`
    (set `self.IsDropping` true)
    (`/Engine/EditorBlueprintResources/StandardMacros.Gate` true :!label _label
      (:`Exit`
        (`|ExecutionSequence`
          (:`then_0`
            (`KismetSystemLibrary.RetriggerableDelay` (`self.MaxHoldTime`))
            (if (`self.IsDropping`)
              (bind _aslast_truck_game_mode (cast `/Game/Blueprints/LastTruckGameMode` (`GameplayStatics.GetGameMode`)))
              (bind _packages (`/Game/Blueprints/LastTruckGameMode.Packages` _aslast_truck_game_mode))
              (if (not (<= _packages 0))
                (bind _result (`/Engine/EditorBlueprintResources/StandardMacros.DecrementInt` _packages)
                  (:`  `
                    (set `/Game/Blueprints/LastTruckGameMode.Packages` _result _aslast_truck_game_mode)
                    (bind _result_2 (`/Engine/EditorBlueprintResources/StandardMacros.IncrementInt` (`/Game/Blueprints/LastTruckGameMode.Pallet1` _aslast_truck_game_mode))
                      (:`  `
                        (set `/Game/Blueprints/LastTruckGameMode.Pallet1` _result_2 _aslast_truck_game_mode)
                        (if (>= (`/Game/Blueprints/LastTruckGameMode.Pallet1` _aslast_truck_game_mode) (`/Game/Blueprints/LastTruckGameMode.MaxPallet1` _aslast_truck_game_mode))
                          (`|SpawnActorFromClass` "/Game/Blueprints/PHCompletePallet.PHCompletePallet_C" (`KismetMathLibrary.Conv_VectorToTransform` (`self.K2_GetActorLocation` (`self.spawnActor`))) "Undefined" "OverrideRootScale" null null)))))))))
          (:`then_1`
            (`self.Timer`)
            (`self.Update Timer`))))))
  (:`Released`
    (set `self.IsDropping` false)))

(event `Stop Timer`
  (`KismetSystemLibrary.K2_PauseTimerHandle` (stale `Timer` _returnvalue)))

(event `Timer`
  (bind _returnvalue (`KismetSystemLibrary.K2_SetTimerDelegate` (delegate `Timer`) (`self.MaxHoldTime`))))

(event `Update Timer`
  (bind _widget (`self.Widget`))
  (if (`self.IsDropping`)
    (set `/Game/Widgets/PalletWidget.TimeHeld` (`KismetSystemLibrary.K2_GetTimerElapsedTimeHandle` (stale `Timer` _returnvalue)) _widget)
    (`KismetSystemLibrary.Delay` 0.1)
    (`self.Update Timer`)
    (else
      (`self.Stop Timer`)
      (set `/Game/Widgets/PalletWidget.TimeHeld` 0.0 _widget))))

(fn `UserConstructionScript`)