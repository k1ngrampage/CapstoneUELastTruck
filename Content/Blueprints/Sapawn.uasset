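; Spawner actor that keeps spawning PlaceholderMonster AI at its root's location, with no population cap.
; On BeginPlay and after each spawn, it counts existing monsters and sets a shorter delay when few exist, longer otherwise.
; Tick drives the repeat through a latent Delay, then spawns and prints a debug message.
; Unconnected leftover nodes, including an alternative delay calculation, never run.
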(event `self.ReceiveBeginPlay`
  (bind _outactors (`GameplayStatics.GetAllActorsOfClass` "/Game/Blueprints/PlaceholderMonster.PlaceholderMonster_C" :!label _label))
  (if (<= (`KismetArrayLibrary.Array_Length` _outactors) 3)
    (set `self.delayTime` 5.0)
    (else
      (set `self.delayTime` 12.0))))

(event `self.ReceiveTick`
  (params (DeltaSeconds :type "Float (single-precision)"))
  (`KismetSystemLibrary.Delay` (`self.delayTime`))
  (`AIBlueprintHelperLibrary.SpawnAIFromClass` "/Game/Blueprints/PlaceholderMonster.PlaceholderMonster_C" null (`SceneComponent.K2_GetComponentLocation` (`self.DefaultSceneRoot`)) (struct) false null)
  (`KismetSystemLibrary.PrintString` "Monster was spawned")
  (goto _label))

(fn `UserConstructionScript`)