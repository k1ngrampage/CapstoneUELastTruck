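; First-person player pawn for Last Truck, with axis-driven movement and look controls that respond to whether pallets are grabbed.
; It reads the grabbed-pallet count from the Last Truck game mode to lower walk speed each Tick and block jumping while carrying.
; Turn and pitch input also move a physics handle target to the camera location.
; Drop input only calls a gate, and placeholder pallet jack spawning is left unconnected.
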(event `self.ReceiveTick`
  (params (DeltaSeconds :type "Float (single-precision)"))
  (bind _charactermovement (`self.CharacterMovement`))
  (if (>= (`/Game/Blueprints/LastTruckGameMode.PalletGrabbed` (`self.LTGMode`)) 1)
    (set `CharacterMovementComponent.MaxWalkSpeed` 300.0 _charactermovement)
    (else
      (set `CharacterMovementComponent.MaxWalkSpeed` 500.0 _charactermovement))))

(event `self.ReceiveHit`
  (params (MyComp :type "PrimitiveComponent Object Reference") (Other :type "Actor Object Reference") (OtherComp :type "PrimitiveComponent Object Reference") (bSelfMoved :type Boolean) (HitLocation :type "Vector Structure") (HitNormal :type "Vector Structure") (NormalImpulse :type "Vector Structure") (Hit :type "HitResult Structure (by ref)")))

(event `self.ReceiveBeginPlay`
  (bind _aslast_truck_game_mode (cast `/Game/Blueprints/LastTruckGameMode` (`GameplayStatics.GetGameMode`)))
  (set `self.LTGMode` _aslast_truck_game_mode))

(event `InputAxis|Move`
  (params (AxisValue :type "Float (single-precision)"))
  (`PawnMovementComponent.AddInputVector` (`self.CharacterMovement`) (* (`self.GetActorForwardVector`) AxisValue) false))

(event `InputAxis|Strafe`
  (params (AxisValue :type "Float (single-precision)"))
  (`PawnMovementComponent.AddInputVector` (`self.CharacterMovement`) (* (`self.GetActorRightVector`) AxisValue) false))

(event `InputAction|Drop`
  (params (Key :type "Key Structure"))
  (:`Pressed`
    (`/Engine/EditorBlueprintResources/StandardMacros.Gate` true)))

(event `InputAction|Jump`
  (params (Key :type "Key Structure"))
  (:`Pressed`
    (if (not (>= (`/Game/Blueprints/LastTruckGameMode.PalletGrabbed` (`self.LTGMode`)) 1))
      (`self.Jump`)))
  (:`Released`
    (`self.StopJumping`)))

(event `InputAxis|Turn`
  (params (AxisValue :type "Float (single-precision)"))
  (bind _camera (`self.Camera`))
  (`self.AddControllerYawInput` AxisValue)
  (`PhysicsHandleComponent.SetTargetLocation` (`self.PhysicsHandle`) (+ (* (`SceneComponent.GetForwardVector` _camera) 0.0) (`SceneComponent.K2_GetComponentLocation` _camera))))

(event `InputAxis|Pitch`
  (params (AxisValue :type "Float (single-precision)"))
  (bind _camera (`self.Camera`))
  (`self.AddControllerPitchInput` AxisValue)
  (`PhysicsHandleComponent.SetTargetLocation` (`self.PhysicsHandle`) (+ (* (`SceneComponent.GetForwardVector` _camera) 0.0) (`SceneComponent.K2_GetComponentLocation` _camera))))

(fn `UserConstructionScript`)