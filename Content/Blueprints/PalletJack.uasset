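; Pallet jack pickup that the player grabs with the Drop input while inside its Box trigger.
; Overlap enables input, opens a gate and shows JackWidget; leaving reverses this and shows PackageWidget.
; Grabbing spawns a replacement jack on the player's Sphere JackSocket, destroys this actor and updates game mode grab count and acquired flag.
; Release only clears the grab flag; pallet contact only prints, and physics-handle logic is unwired.
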(event `InputAction|Drop`
  (params (Key :type "Key Structure"))
  (bind _sphere (`/Game/Blueprints/LastTruckPlayerPawn.Sphere` (`self.Player`)))
  (:`Pressed`
    (set `self.IsGrabbed` true)
    (`KismetSystemLibrary.PrintString` "Active Grab")
    (`/Engine/EditorBlueprintResources/StandardMacros.Gate` true :!label _label
      (:`Exit`
        (if (`self.IsGrabbed`)
          (`/Engine/EditorBlueprintResources/StandardMacros.IncrementInt` (`/Game/Blueprints/LastTruckGameMode.PalletGrabbed` (`self.LTGMode`))
            (:`  `
              (bind _returnvalue (`|SpawnActorFromClass` "PalletJack_C" (`SceneComponent.GetSocketTransform` _sphere "JackSocket" "RTS_World") "Undefined" "OverrideRootScale" null null))
              (bind _output_get (set `self.PalletJack` _returnvalue))
              (`self.K2_AttachToComponent` _output_get _sphere "JackSocket" "SnapToTarget" "SnapToTarget" "SnapToTarget" true)
              (`self.K2_DestroyActor`)
              (set `/Game/Blueprints/LastTruckGameMode.PalletJackAcquired` true (`self.LTGMode`))))))))
  (:`Released`
    (set `self.IsGrabbed` false)
    (`KismetSystemLibrary.PrintString` "Not grabbed")))

(event `self.Box.OnComponentBeginOverlap`
  (params (OverlappedComponent :type "PrimitiveComponent Object Reference") (OtherActor :type "Actor Object Reference") (OtherComp :type "PrimitiveComponent Object Reference") (OtherBodyIndex :type Integer) (bFromSweep :type Boolean) (SweepResult :type "HitResult Structure (by ref)"))
  (cast `/Game/Blueprints/LastTruckPlayerPawn` OtherActor)
  (`self.EnableInput` (`GameplayStatics.GetPlayerController` 0))
  (bind _returnvalue (`|CreateWidget` "/Game/Widgets/JackWidget.JackWidget_C"))
  (`UserWidget.AddToViewport` _returnvalue 0)
  (goto _label :!via `Open`))

(event `self.ReceiveBeginPlay`
  (bind _aslast_truck_player_pawn (cast `/Game/Blueprints/LastTruckPlayerPawn` (`GameplayStatics.GetPlayerPawn` 0)))
  (set `self.Player` _aslast_truck_player_pawn)
  (bind _aslast_truck_game_mode (cast `/Game/Blueprints/LastTruckGameMode` (`GameplayStatics.GetGameMode`)))
  (set `self.LTGMode` _aslast_truck_game_mode))

(event `self.Box.OnComponentEndOverlap`
  (params (OverlappedComponent :type "PrimitiveComponent Object Reference") (OtherActor :type "Actor Object Reference") (OtherComp :type "PrimitiveComponent Object Reference") (OtherBodyIndex :type Integer))
  (cast `/Game/Blueprints/LastTruckPlayerPawn` OtherActor)
  (`self.DisableInput` (`GameplayStatics.GetPlayerController` 0))
  (`WidgetLayoutLibrary.RemoveAllWidgets`)
  (bind _returnvalue (`|CreateWidget` "/Game/Widgets/PackageWidget.PackageWidget_C"))
  (`UserWidget.AddToViewport` _returnvalue 0)
  (goto _label :!via `Close`))

(event `InputAction|DropPallet`
  (params (Key :type "Key Structure")))

(event `self.Box1.OnComponentBeginOverlap`
  (params (OverlappedComponent :type "PrimitiveComponent Object Reference") (OtherActor :type "Actor Object Reference") (OtherComp :type "PrimitiveComponent Object Reference") (OtherBodyIndex :type Integer) (bFromSweep :type Boolean) (SweepResult :type "HitResult Structure (by ref)"))
  (cast `/Game/Blueprints/PHCompletePallet` OtherActor)
  (`KismetSystemLibrary.PrintString` "Pushing pallet"))

(fn `UserConstructionScript`)