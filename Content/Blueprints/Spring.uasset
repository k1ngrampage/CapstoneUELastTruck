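; Spring actor that launches whatever hits it along its up axis, acting as a bounce pad.
; On Hit, it checks that the negated hit normal closely aligns with the actor's up vector, then applies a SpringPower-scaled force along that negated normal.
; LastTruckPlayerPawn receives the force through CharacterMovement with a 2D hop sound; anything else receives it on the hit component.
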(event `self.ReceiveHit`
  (params (MyComp :type "PrimitiveComponent Object Reference") (Other :type "Actor Object Reference") (OtherComp :type "PrimitiveComponent Object Reference") (bSelfMoved :type Boolean) (HitLocation :type "Vector Structure") (HitNormal :type "Vector Structure") (NormalImpulse :type "Vector Structure") (Hit :type "HitResult Structure (by ref)"))
  (bind _returnvalue (`KismetMathLibrary.NegateVector` HitNormal))
  (bind _returnvalue_2 (* _returnvalue (`self.SpringPower`)))
  (if (> (`KismetMathLibrary.Dot_VectorVector` _returnvalue (`self.GetActorUpVector`)) 0.8)
    (bind _aslast_truck_player_pawn (cast `/Game/Blueprints/LastTruckPlayerPawn` Other)
      (:`then`
        (`CharacterMovementComponent.AddForce` (`Character.CharacterMovement` _aslast_truck_player_pawn) _returnvalue_2)
        (`GameplayStatics.SpawnSound2D` "/Game/Audio/jump_hop_by_felixyadomi.jump_hop_by_felixyadomi" 1.0 1.0 0.0 null))
      (:`CastFailed`
        (`PrimitiveComponent.AddForce` OtherComp _returnvalue_2 "None" false)))))

(fn `UserConstructionScript`)