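; Placeholder ghost monster for the Last Truck game that loads LoseLevel when it hits the player pawn.
; Tick wanders it to random reachable points after short random delays and turns it toward its velocity, while PawnSensing sends it after a seen player.
; BeginPlay destroys it after a default Lifespan delay.
; Tick rescales Lifespan by the game mode's package count, but only after that delay has started.
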(event `self.ReceiveTick`
  (params (DeltaSeconds :type "Float (single-precision)"))
  (bind _returnvalue (`KismetMathLibrary.Conv_IntToDouble` (`/Game/Blueprints/LastTruckGameMode.Packages` (`self.LTGMode`))))
  (`KismetSystemLibrary.Delay` (`KismetMathLibrary.RandomFloatInRange` 1.0 3.0))
  (set `self.isMoving` true)
  (`KismetSystemLibrary.PrintString` "Is Moving")
  (`|AIMoveTo` self (`NavigationSystemV1.K2_GetRandomReachablePointInRadius` (`self.K2_GetActorLocation`) 1500.0 null null) null
    (:`then`
      (`self.Rotate to Face Direction` (`MovementComponent.Velocity` (`self.FloatingPawnMovement`)))
      (if (== _returnvalue 1.0)
        (set `self.Lifespan` 12.0)
        (elif (== _returnvalue 2.0)
          (set `self.Lifespan` 16.0)
          (elif (== _returnvalue 3.0)
            (set `self.Lifespan` 25.0)))))
    (:`OnSuccess`
      (set `self.isMoving` false :!label _label))
    (:`OnFail`
      (goto _label))))

(event `self.ReceiveBeginPlay`
  (set `self.Lifespan` 8.0)
  (bind _aslast_truck_game_mode (cast `/Game/Blueprints/LastTruckGameMode` (`GameplayStatics.GetGameMode`)))
  (set `self.LTGMode` _aslast_truck_game_mode)
  (`KismetSystemLibrary.Delay` (`self.Lifespan`))
  (`self.K2_DestroyActor`)
  (`KismetSystemLibrary.PrintString` "Ghost disappeared lol"))

(event `self.ReceiveHit`
  (params (MyComp :type "PrimitiveComponent Object Reference") (Other :type "Actor Object Reference") (OtherComp :type "PrimitiveComponent Object Reference") (bSelfMoved :type Boolean) (HitLocation :type "Vector Structure") (HitNormal :type "Vector Structure") (NormalImpulse :type "Vector Structure") (Hit :type "HitResult Structure (by ref)"))
  (cast `/Game/Blueprints/LastTruckPlayerPawn` Other)
  (`GameplayStatics.OpenLevel` "LoseLevel"))

(event `self.PawnSensing.OnSeePawn`
  (params (Pawn :type "Pawn Object Reference"))
  (bind _aslast_truck_player_pawn (cast `/Game/Blueprints/LastTruckPlayerPawn` Pawn))
  (`|ExecutionSequence`
    (:`then_0`
      (set `self.EnemySpotted` true)
      (`|AIMoveTo` self (0.0 0.0 0.0) _aslast_truck_player_pawn))
    (:`then_1`
      (set `self.EnemySpotted` false))))

(fn `Rotate to Face Direction`
  (params (Direction :type "Vector Structure"))
  (locals (DirectionXYZ :type "Vector Structure"))
  (set `local.DirectionXYZ` (`KismetMathLibrary.MakeVector` Direction_X Direction_Y Direction_Z))
  (`self.K2_SetActorRotation` (`KismetMathLibrary.MakeRotFromX` (`local.DirectionXYZ`))))

(fn `UserConstructionScript`)