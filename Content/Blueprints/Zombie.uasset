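; Zombie enemy pawn that wanders the navmesh and moves toward the LastTruck player pawn when PawnSensing sees it.
; Tick uses a random Delay to pace AIMoveTo calls to random reachable nearby points, yawing the actor toward its movement velocity after issuing each move.
; EnemySpotted and IsMoving are set but never read here.
; Hit only casts to the player, as the sound, life-loss and destroy nodes are disconnected.
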(event `self.ReceiveHit`
  (params (MyComp :type "PrimitiveComponent Object Reference") (Other :type "Actor Object Reference") (OtherComp :type "PrimitiveComponent Object Reference") (bSelfMoved :type Boolean) (HitLocation :type "Vector Structure") (HitNormal :type "Vector Structure") (NormalImpulse :type "Vector Structure") (Hit :type "HitResult Structure (by ref)"))
  (cast `/Game/Blueprints/LastTruckPlayerPawn` Other))

(event `self.ReceiveTick`
  (params (DeltaSeconds :type "Float (single-precision)"))
  (`KismetSystemLibrary.Delay` (`KismetMathLibrary.RandomFloatInRange` 1.0 3.0))
  (set `self.isMoving` true)
  (`|AIMoveTo` self (`NavigationSystemV1.K2_GetRandomReachablePointInRadius` (`self.K2_GetActorLocation`) 1500.0 null null) null
    (:`then`
      (`self.RotateToFaceDirection` (`MovementComponent.Velocity` (`self.FloatingPawnMovement`))))
    (:`OnSuccess`
      (set `self.isMoving` false :!label _label))
    (:`OnFail`
      (goto _label))))

(event `self.PawnSensing.OnSeePawn`
  (params (Pawn :type "Pawn Object Reference"))
  (bind _aslast_truck_player_pawn (cast `/Game/Blueprints/LastTruckPlayerPawn` Pawn))
  (`|ExecutionSequence`
    (:`then_0`
      (set `self.EnemySpotted` true)
      (`|AIMoveTo` self (0.0 0.0 0.0) _aslast_truck_player_pawn))
    (:`then_1`
      (set `self.EnemySpotted` false))))

(fn `RotateToFaceDirection`
  (params (Direction :type "Vector Structure"))
  (locals (DirectionXY :type "Vector Structure"))
  (set `local.DirectionXY` (`KismetMathLibrary.MakeVector` Direction_X Direction_Y))
  (`self.K2_SetActorRotation` (`KismetMathLibrary.MakeRotFromX` (`local.DirectionXY`))))

(fn `UserConstructionScript`)